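; World catastrophes manager actor that tracks world health, signals catastrophes and handles the game-over transition.
; On BeginPlay it caches the main game widget after a short delay, then pushes WorldStatsComponent health to the EcoBot world bar through OnStatsChange.
; OnCatastrophe plays a sound and shows its directional light for a timed period.
; Die waits briefly, then opens the GameOverMenu level.
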(event `self.ReceiveBeginPlay`
  (bind (_healthstat_statname _healthstat_maxvalue _healthstat_currentvalue _healthstat_percentvalue) (break `Stat` (`EcoBotStatsComponent.HealthStat` (`self.WorldStatsComponent`))))
  (`KismetSystemLibrary.Delay` 0.25)
  (`self.ReferenceMainWidget`)
  (`self.OnStatsChange` _healthstat_percentvalue))

(event `self.OnStatsChange`
  (params (HealthPercent :type "Float (single-precision)") (HungerPercent :type "Float (single-precision)") (ThirstPercent :type "Float (single-precision)"))
  (if (`KismetSystemLibrary.IsValid` (`self.MainWidget`))
    (`/Game/Blueprints/Widgets/InGame/BP_EcoBotWidget.UpdateWorldBar` (`/Game/Blueprints/Widgets/InGame/BP_MainGameWidget.EcoBotWidget` (`self.MainWidget`)) HealthPercent)
    (else
      (`self.ReferenceMainWidget`))))

(event `self.OnCatastrophe`
  (`GameplayStatics.PlaySound2D` "/Game/Blueprints/Audio/MetaSounds/MS_Catastrophe.MS_Catastrophe" 1.0 1.0 0.0 null null)
  (`SceneComponent.SetVisibility` (`self.DirectionalLight`) true true)
  (`KismetSystemLibrary.Delay` 10.0)
  (`SceneComponent.SetVisibility` (`self.DirectionalLight`) false false))

(event `self.Die`
  (`KismetSystemLibrary.Delay` 4.0)
  (`GameplayStatics.OpenLevelBySoftObjectPtr` "/Game/Levels/Menu/GameOverMenu.GameOverMenu"))

(fn `ReferenceMainWidget`
  (bind _foundwidgets (`WidgetBlueprintLibrary.GetAllWidgetsOfClass` "/Game/Blueprints/Widgets/InGame/BP_MainGameWidget.BP_MainGameWidget_C" false))
  (for _array_element _foundwidgets
    (set `self.MainWidget` _array_element)))

(fn `UserConstructionScript`)