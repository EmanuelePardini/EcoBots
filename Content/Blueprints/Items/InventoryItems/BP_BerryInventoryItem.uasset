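; Inventory item for a berry that an EcoBot character can eat to restore hunger and possibly health.
; Using the item calls EatBerry, which raises the character's hunger stat through its StatsComponent and then calls Heal.
; Heal restores health only when both the thirst and hunger stats are at their maximum values.
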(event `self.OnUseInventoryItem`
  (params (EcoBotCharacter :type "EcoBotCharacter Object Reference"))
  (`self.EatBerry` EcoBotCharacter))

(fn `EatBerry`
  (params (InteractingChar :type "EcoBotCharacter Object Reference"))
  (`EcoBotStatsComponent.IncrementHunger` (`EcoBotCharacter.StatsComponent` InteractingChar) 100.0)
  (`self.Heal` InteractingChar))

(fn `Heal`
  (params (InteractingChar :type "EcoBotCharacter Object Reference"))
  (bind _statscomponent (`EcoBotCharacter.StatsComponent` InteractingChar))
  (bind (_hungerstat_statname _hungerstat_maxvalue _hungerstat_currentvalue) (break `Stat` (`EcoBotStatsComponent.HungerStat` _statscomponent)))
  (bind (_thirststat_statname _thirststat_maxvalue _thirststat_currentvalue) (break `Stat` (`EcoBotStatsComponent.ThirstStat` _statscomponent)))
  (if (and (>= _thirststat_currentvalue _thirststat_maxvalue) (>= _hungerstat_currentvalue _hungerstat_maxvalue))
    (`EcoBotStatsComponent.IncrementHealth` _statscomponent 100.0)))