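; BP_Water is an interactable water volume that puts EcoBot characters into a flying state while they overlap it.
; On overlap begin it casts the actor to BP_EcoBotCharacter or BP_EcoBotBuddy, sets IsFlying on its anim instance and shows its JetPackVFX.
; On overlap end it clears the flag and hides the VFX, without propagating the hide to child components.
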(event `self.ReceiveActorBeginOverlap`
  (params (OtherActor :type "Actor Object Reference"))
  (bind _asbp_eco_bot_character (cast `/Game/Blueprints/Characters/BP_EcoBotCharacter` OtherActor)
    (:`then`
      (bind _returnvalue (`EcoBotCharacter.GetEcoBotAnim` _asbp_eco_bot_character))
      (set `EcoBotAnim.IsFlying` true _returnvalue)
      (`SceneComponent.SetVisibility` (`/Game/Blueprints/Characters/BP_EcoBotCharacter.JetPackVFX` _asbp_eco_bot_character) true true))
    (:`CastFailed`
      (bind _asbp_eco_bot_buddy (cast `/Game/Blueprints/Characters/AI/BP_EcoBotBuddy` OtherActor))
      (bind _returnvalue_2 (`EcoBotCharacter.GetEcoBotAnim` _asbp_eco_bot_buddy))
      (set `EcoBotAnim.IsFlying` true _returnvalue_2)
      (`SceneComponent.SetVisibility` (`/Game/Blueprints/Characters/AI/BP_EcoBotBuddy.JetPackVFX` _asbp_eco_bot_buddy) true true))))

(event `self.ReceiveActorEndOverlap`
  (params (OtherActor :type "Actor Object Reference"))
  (bind _asbp_eco_bot_character (cast `/Game/Blueprints/Characters/BP_EcoBotCharacter` OtherActor)
    (:`then`
      (bind _returnvalue (`EcoBotCharacter.GetEcoBotAnim` _asbp_eco_bot_character))
      (set `EcoBotAnim.IsFlying` false _returnvalue)
      (`SceneComponent.SetVisibility` (`/Game/Blueprints/Characters/BP_EcoBotCharacter.JetPackVFX` _asbp_eco_bot_character) false false))
    (:`CastFailed`
      (bind _asbp_eco_bot_buddy (cast `/Game/Blueprints/Characters/AI/BP_EcoBotBuddy` OtherActor))
      (bind _returnvalue_2 (`EcoBotCharacter.GetEcoBotAnim` _asbp_eco_bot_buddy))
      (set `EcoBotAnim.IsFlying` false _returnvalue_2)
      (`SceneComponent.SetVisibility` (`/Game/Blueprints/Characters/AI/BP_EcoBotBuddy.JetPackVFX` _asbp_eco_bot_buddy) false false))))

(fn `UserConstructionScript`)