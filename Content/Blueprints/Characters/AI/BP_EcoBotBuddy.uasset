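; BP_EcoBotBuddy is a buddy robot that shows phrases and talks when another EcoBotCharacter comes near.
; On BeginPlay it caches its BP_BuddyPhrasesWidget from the widget component and hides it.
; A Box overlap by an EcoBotCharacter other than itself calls the widget's ManagePhrasesWidget, plays a robot talk sound at the buddy's location, then hides the widget after a short delay.
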(event `self.ReceiveBeginPlay`
  (bind _asbp_buddy_phrases_widget (cast `/Game/Blueprints/Widgets/InGame/BP_BuddyPhrasesWidget` (`WidgetComponent.GetUserWidgetObject` (`self.PhrasesWidget`))))
  (bind _output_get (set `self.PhrasesWidgetRef` _asbp_buddy_phrases_widget))
  (`Widget.SetVisibility` _output_get "Hidden"))

(event `self.ReceiveTick`
  (params (DeltaSeconds :type "Float (single-precision)")))

(event `self.Box.OnComponentBeginOverlap`
  (params (OverlappedComponent :type "PrimitiveComponent Object Reference") (OtherActor :type "Actor Object Reference") (OtherComp :type "PrimitiveComponent Object Reference") (OtherBodyIndex :type Integer) (bFromSweep :type Boolean) (SweepResult :type "HitResult Structure (by ref)"))
  (bind _phraseswidgetref (`self.PhrasesWidgetRef`))
  (bind _aseco_bot_character (cast `EcoBotCharacter` OtherActor))
  (if (!= _aseco_bot_character self)
    (`/Game/Blueprints/Widgets/InGame/BP_BuddyPhrasesWidget.ManagePhrasesWidget` _phraseswidgetref)
    (`GameplayStatics.PlaySoundAtLocation` "/Game/Blueprints/Audio/MetaSounds/MS_RobotTalk.MS_RobotTalk" (`self.K2_GetActorLocation`) (struct) 1.0 1.0 0.0 null null null null)
    (`KismetSystemLibrary.Delay` 5.0)
    (`Widget.SetVisibility` _phraseswidgetref "Hidden")))

(fn `UserConstructionScript`)