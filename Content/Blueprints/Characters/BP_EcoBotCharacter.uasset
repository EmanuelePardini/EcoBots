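; EcoBot character Blueprint that links the character's gameplay events to UI, audio and particle feedback.
; Inventory, stat and crafting events update sub-widgets of a cached main game widget, re-fetched when invalid; Escape or P manages the pause widget.
; Interaction toggles particles and plays a sound on start, while sphere overlaps show or hide a prompt for Interactable actors or component owners.
; Death opens the game-over level after a short delay.
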(event `self.ReceiveBeginPlay`
  (`self.ReferenceMainWidget`))

(event `self.OnInventoryChanged`
  (params (Slots :type "Array of InventorySlot Object Reference (by ref)"))
  ;[1 1 1] On Inventory Update
  (if (not (`KismetSystemLibrary.IsValid` (`self.WidgetRef`)))
    (`self.ReferenceMainWidget`))
  (`/Game/Blueprints/Widgets/InGame/BP_InventoryWidget.UpdateInventory` (`/Game/Blueprints/Widgets/InGame/BP_MainGameWidget.InventoryWidget` (`self.WidgetRef`)) Slots))

(event `self.OnCraftChanged`
  (params (CraftRecipes :type "Array of CraftRecipe Object Reference (by ref)"))
  ;[1 1 1] Update Craft Component
  (if (not (`KismetSystemLibrary.IsValid` (`self.WidgetRef`)))
    (`self.ReferenceMainWidget`))
  (`/Game/Blueprints/Widgets/InGame/BP_CraftWidget.UpdateCraft` (`/Game/Blueprints/Widgets/InGame/BP_MainGameWidget.CraftWidget` (`self.WidgetRef`)) CraftRecipes))

(event `self.OnStatsChange`
  (params (HealthPercent :type "Float (single-precision)") (HungerPercent :type "Float (single-precision)") (ThirstPercent :type "Float (single-precision)"))
  ;[1 1 1] Update UI Stats
  (if (not (`KismetSystemLibrary.IsValid` (`self.WidgetRef`)))
    (`self.ReferenceMainWidget`))
  (`/Game/Blueprints/Widgets/InGame/BP_EcoBotWidget.UpdateBars` (`/Game/Blueprints/Widgets/InGame/BP_MainGameWidget.EcoBotWidget` (`self.WidgetRef`)) HealthPercent HungerPercent ThirstPercent))

(event `CustomEvent`
  (params (CraftRecipes :type "Array of CraftRecipe Object Reference (by ref)")))

(event `Key|Escape` :paused true
  (params (Key :type "Key Structure"))
  ;[1 1 1] Manage Pause
  (:`Released`
    (`/Game/Blueprints/Widgets/InGame/BP_PauseWidget.ManagePause` (`/Game/Blueprints/Widgets/InGame/BP_MainGameWidget.PauseWidget` (`self.WidgetRef`)) :!label _label)))

(event `Key|P`
  (params (Key :type "Key Structure"))
  ;[1 1 1] Manage Pause
  (:`Released`
    (goto _label)))

(event `self.Die`
  ;[1 1 1] Die Manage
  (`KismetSystemLibrary.Delay` 4.0)
  (`GameplayStatics.OpenLevelBySoftObjectPtr` "/Game/Levels/Menu/GameOverMenu.GameOverMenu"))

(event `self.OnBeginInteract`
  ;[1 1 1] Interaction Manage
  (`SceneComponent.SetVisibility` (`self.InteractionParticle`) true true)
  (`SceneComponent.SetVisibility` (`self.InteractionParticle`) true true)
  (`GameplayStatics.PlaySoundAtLocation` "/Game/Blueprints/Audio/MetaSounds/MS_RobotInteract.MS_RobotInteract" (`self.K2_GetActorLocation`) (struct) 1.0 1.0 0.0 null null null null))

(event `self.OnEndInteract`
  ;[1 1 1] Interaction Manage
  (`SceneComponent.SetVisibility` (`self.InteractionParticle`) false false)
  (`SceneComponent.SetVisibility` (`self.InteractionParticle`) false false))

(event `self.InteractionSphere.OnComponentBeginOverlap`
  (params (OverlappedComponent :type "PrimitiveComponent Object Reference") (OtherActor :type "Actor Object Reference") (OtherComp :type "PrimitiveComponent Object Reference") (OtherBodyIndex :type Integer) (bFromSweep :type Boolean) (SweepResult :type "HitResult Structure (by ref)"))
  ;[1 1 1] Manage Interaction Widget
  (`self.ManageInteractionWidget` true OtherActor))

(event `self.InteractionSphere.OnComponentEndOverlap`
  (params (OverlappedComponent :type "PrimitiveComponent Object Reference") (OtherActor :type "Actor Object Reference") (OtherComp :type "PrimitiveComponent Object Reference") (OtherBodyIndex :type Integer))
  ;[1 1 1] Manage Interaction Widget
  (`self.ManageInteractionWidget` false OtherActor))

(fn `ManageInteractionWidget`
  (params (VisibilityToSet :type Boolean) (Interactable :type "Actor Object Reference"))
  (cast `Interactable` Interactable
    (:`then`
      (`SceneComponent.SetVisibility` (`self.InteractionWidget`) VisibilityToSet true :!label _label))
    (:`CastFailed`
      (if (`KismetSystemLibrary.IsValid` (`self.GetComponentByClass` Interactable "/Script/EcoBots.InteractableComponent"))
        (goto _label)))))

(fn `ReferenceMainWidget`
  (bind _asbp_main_game_widget (cast `/Game/Blueprints/Widgets/InGame/BP_MainGameWidget` (`self.EcoBotWidgetInstance`)))
  (set `self.WidgetRef` _asbp_main_game_widget))

(fn `UserConstructionScript`)