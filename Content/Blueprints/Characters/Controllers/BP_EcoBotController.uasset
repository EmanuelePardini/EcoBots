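; BP_EcoBotController is the EcoBot character's controller, handling the game's pause menu.
; On BeginPlay it creates a BP_PauseWidget, adds it to the viewport hidden and keeps a reference to it.
; Releasing Escape or P calls ManagePause, which toggles the game's paused state and shows or hides that widget to match.
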(event `self.ReceiveBeginPlay`
  ;[1 1 1] Pause Widget reference
  (bind _returnvalue (`|CreateWidget` "/Game/Blueprints/Widgets/InGame/BP_PauseWidget.BP_PauseWidget_C"))
  (`Widget.SetVisibility` _returnvalue "Hidden")
  (`UserWidget.AddToViewport` _returnvalue 0)
  (set `self.PauseWidgetRef` _returnvalue))

(event `Key|Escape` :paused true
  (params (Key :type "Key Structure"))
  (:`Released`
    (`self.ManagePause` :!label _label)))

(event `Key|P`
  (params (Key :type "Key Structure"))
  (:`Released`
    (goto _label)))

(fn `ManagePause`
  (if (`GameplayStatics.IsGamePaused`)
    (`GameplayStatics.SetGamePaused` false)
    (`Widget.SetVisibility` (`self.PauseWidgetRef`) "Hidden")
    (else
      (`GameplayStatics.SetGamePaused` true)
      (`Widget.SetVisibility` (`self.PauseWidgetRef`) "Visible"))))

(fn `UserConstructionScript`)